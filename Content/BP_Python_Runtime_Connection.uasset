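; Blueprint TCP client that links the running game to a Python server, opened through StartPythonConnection or NumPad 1.
; Connect, disconnect and receive callbacks track the connection ID and connected state, with optional on-screen debug messages.
; Outgoing strings are sent as bytes; incoming bytes become a stored string that is passed on through IncomingDataFromPython.
; Helper functions expose disconnecting and a connection-status check.
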(event Custom|Start%20Python%20Connection
  (bind _connectionid (Class|TcpSocketConnection|Connect (Variables|SocketConnection|GetIp%20Address) (Variables|SocketConnection|GetPort) (|HandleDisconnectfromPython) (|HandleConnectionToPython) (|HandleRecievingDataFromPython)))
  (Variables|SocketConnection|SetConnection%20Id _connectionid))

(event Input|KeyboardEvents|NumPadOne
  (params (Key :type Key%20Structure))
  ;[0.111 0.4219 0] Start or Retry Connection
  (:Pressed
    (CallFunction|StartPythonConnection)))

(fn ConstructionScript)

(fn SendDatatoPyScript
  (params (Data%20as%20Strng :type String))
  (bind _returnvalue (Class|TcpSocketConnection|SendData (Variables|SocketConnection|GetConnection%20Id) (Class|TcpSocketConnection|ToBytes(String) Data%20as%20Strng)))
  (if (Variables|PythonDebugging|GetDebugging%20Enabled)
    (Development|PrintString (Utilities|String|ToString(Text) (Utilities|Text|FormatText "Data Sending was {status}" _returnvalue)) true true "(R=1.000000,G=1.000000,B=0.000000,A=1.000000)" 1e+01 "sdfdv"))
  (return _returnvalue))

(fn DisconnectfromPython
  (Class|TcpSocketConnection|Disconnect (Variables|SocketConnection|GetConnection%20Id))
  (Variables|SocketConnection|SetConnection%20Id 0))

(fn CheckPythonConnected
  (return (Variables|SocketConnection|GetConnected%20To%20Python)))

(event Custom|Disconnected
  (params (ConnectionId :type Integer))
  ;[1 1 1] When Disconnected From TCP Server
  (Class|TcpSocketConnection|Disconnect (Variables|SocketConnection|GetConnection%20Id))
  (Variables|SocketConnection|SetConnection%20Id 0)
  (Variables|SocketConnection|SetConnected%20To%20Python false)
  (if (Variables|PythonDebugging|GetDebugging%20Enabled)
    (Development|PrintString (Utilities|String|Append "Warning! Python Server Connection {" (Utilities|String|ToString(Integer) (Variables|SocketConnection|GetConnection%20Id)) "} Has Disconnected!") true true "(R=1.000000,G=1.000000,B=0.000000,A=1.000000)" 1e+01)))

(event Custom|Connected
  (params (ConnectionId :type Integer))
  ;[1 1 1] When Connection Successful To Server
  (Variables|SocketConnection|SetConnected%20To%20Python true)
  (Variables|SocketConnection|SetConnection%20Id ConnectionId)
  (if (Variables|PythonDebugging|GetDebugging%20Enabled)
    (Development|PrintString (Utilities|String|ToString(Text) (Utilities|Text|FormatText "Connected To Python Successfully;;  IP: {IP},  PORT: {PORT},  CONN_ID: {ID}  " (Variables|SocketConnection|GetIp%20Address) (Variables|SocketConnection|GetPort) (Variables|SocketConnection|GetConnection%20Id))) true true "(R=0.247933,G=1.000000,B=0.000000,A=1.000000)" 2e+01 "dfgds")))

(event Custom|TCP%20Recieved
  (params (ConnectionId :type Integer) (Message :type Array%20of%20Bytes))
  ;[1 1 1] On Recieved Data From TCP Server
  (bind _returnvalue (Class|PythonFunctionLibrary|ConvertBytestoString Message))
  (Variables|Data|SetRecieved%20Data _returnvalue)
  (if (Variables|PythonDebugging|GetDebugging%20Enabled)
    (Development|PrintString (Utilities|String|ToString(Text) (Utilities|Text|FormatText "Incoming Data Recieved from;;  IP: {ip},  PORT: {port},  CONN_ID:  {con_id}" (Variables|SocketConnection|GetIp%20Address) (Variables|SocketConnection|GetPort) (Variables|SocketConnection|GetConnection%20Id))) true true "(R=0.000000,G=1.000000,B=0.000000,A=1.000000)" 1e+01 "dsfvss"))
  (Default|CallIncomingDatafromPython (Variables|Data|GetRecieved%20Data)))